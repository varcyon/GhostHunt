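; Configurable classic bus prop whose look is set entirely in the Construction Script, with no active runtime logic.
; Front, back and driver door values scale yaw rotations to pose the door meshes.
; With CustomMaterials on, it creates dynamic material instances, shares body and glass ones with the doors, then sets paint colours, finishes, pattern mask, rust, dirt, wipers and wheel discs.
; Front, back and turn-side lights are toggled through body material parameters.
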(event EventBeginPlay)

(event Collision|EventActorBeginOverlap
  (params (OtherActor :type Actor%20Object%20Reference)))

(event EventTick
  (params (DeltaSeconds :type Float%20%28single-precision%29)))

(fn ConstructionScript
  (Doors|FrontDoorAction (Variables|Doors|GetFrontDoors))
  (Doors|BackDoorActions (Variables|Doors|GetBackDoors))
  (Doors|DriverDoorAction (Variables|Doors|GetDriver_Door))
  (if (Variables|Customization|GetCustomMaterials)
    (Customization|GenerateDynamicMat)
    (Customization|MaterialSetting)
    (Customization|CarLights (Variables|Light|GetFrontLight) (Variables|Light|GetBackLights) (Variables|Light|GetRightLights) (Variables|Light|GetLightLights))))

(fn FrontDoorAction
  (params (OpenCoof :type Float%20%28single-precision%29))
  (Transformation|SetRelativeRotation (Variables|Default|GetFrontPosDoor03) (Math|Rotator|MakeRotator 0.0 0.0 (* 75.0 OpenCoof)) false false)
  (Transformation|SetRelativeRotation (Variables|Default|GetFrontPosDoor04) (Math|Rotator|MakeRotator 0.0 0.0 (* -175.0 OpenCoof)) false false)
  (Transformation|SetRelativeRotation (Variables|Default|GetFrontPosDoor01) (Math|Rotator|MakeRotator 0.0 0.0 (* -75.0 OpenCoof)) false false)
  (Transformation|SetRelativeRotation (Variables|Default|GetFrontPosDoor02) (Math|Rotator|MakeRotator 0.0 0.0 (* 175.0 OpenCoof)) false false)
  (return))

(fn BackDoorActions
  (params (OpenCoof :type Float%20%28single-precision%29))
  (Transformation|SetRelativeRotation (Variables|Default|GetBackPosDoor04) (Math|Rotator|MakeRotator 0.0 0.0 (* 75.0 OpenCoof)) false false)
  (Transformation|SetRelativeRotation (Variables|Default|GetBackPosDoor03) (Math|Rotator|MakeRotator 0.0 0.0 (* -175.0 OpenCoof)) false false)
  (Transformation|SetRelativeRotation (Variables|Default|GetBackPosDoor01) (Math|Rotator|MakeRotator 0.0 0.0 (* -75.0 OpenCoof)) false false)
  (Transformation|SetRelativeRotation (Variables|Default|GetBackPosDoor02) (Math|Rotator|MakeRotator 0.0 0.0 (* 175.0 OpenCoof)) false false)
  (return))

(fn DriverDoorAction
  (params (DriverDoor :type Float%20%28single-precision%29))
  (bind _relativerotation (Variables|/Script/Engine.SceneComponent|GetRelativeRotation (Variables|Default|GetDriverDoor)))
  (bind (_roll _pitch) (Math|Rotator|BreakRotator _relativerotation))
  (Transformation|SetRelativeRotation (Variables|Default|GetDriverDoor) (Math|Rotator|MakeRotator _roll _pitch (* DriverDoor 6e+01)) false false)
  (return))

(fn GenerateDynamicMat
  (bind _body (Variables|Default|GetBody))
  (bind _under (Variables|Default|GetUnder))
  (bind _wheels (Variables|Default|GetWheels))
  (bind _in (Variables|Default|GetIn))
  (bind _driverdoor (Variables|Default|GetDriverDoor))
  (bind _returnvalue (Rendering|Material|CreateDynamicMaterialInstance _body 0 (Rendering|Material|GetMaterial _body 0) :!class /Script/Engine.PrimitiveComponent))
  (Variables|DymamicMat|SetBodyDynamic _returnvalue)
  (bind _returnvalue_2 (Rendering|Material|CreateDynamicMaterialInstance _body 1 (Rendering|Material|GetMaterial _body 1) :!class /Script/Engine.PrimitiveComponent))
  (Variables|DymamicMat|SetGlassDynamic _returnvalue_2)
  (bind _returnvalue_3 (Rendering|Material|CreateDynamicMaterialInstance _wheels 0 (Rendering|Material|GetMaterial _wheels 0) :!class /Script/Engine.PrimitiveComponent))
  (Variables|DymamicMat|SetWheelsDynamic _returnvalue_3)
  (bind _returnvalue_4 (Rendering|Material|CreateDynamicMaterialInstance _under 0 (Rendering|Material|GetMaterial _under 0) :!class /Script/Engine.PrimitiveComponent))
  (Variables|DymamicMat|SetUnderDynamic _returnvalue_4)
  (bind _returnvalue_5 (Rendering|Material|CreateDynamicMaterialInstance _in 0 (Rendering|Material|GetMaterial _in 0) :!class /Script/Engine.PrimitiveComponent))
  (Variables|DymamicMat|SetInDynamic _returnvalue_5)
  (Rendering|Material|SetMaterial _driverdoor 0 (Variables|DymamicMat|GetBodyDynamic))
  (Rendering|Material|SetMaterial _driverdoor 0 (Variables|DymamicMat|GetBodyDynamic))
  (Rendering|Material|SetMaterial _driverdoor 1 (Variables|DymamicMat|GetGlassDynamic))
  (Rendering|Material|SetMaterial _driverdoor 1 (Variables|DymamicMat|GetGlassDynamic))
  (return))

(fn MaterialSetting
  (bind _bodydynamic (Variables|DymamicMat|GetBodyDynamic))
  (bind _basecolortype (Variables|Customization|GetBaseColorType))
  (bind _secondcolortype (Variables|Customization|GetSecondColorType))
  (bind _bodydynamic_2 (Variables|DymamicMat|GetBodyDynamic))
  (bind _wheelsdynamic (Variables|DymamicMat|GetWheelsDynamic))
  (bind _wheeldisc (Variables|Customization|GetWheelDisc))
  (Rendering|Material|SetVectorParameterValue _bodydynamic "FirstColor" (Variables|Customization|GetBaseColor) :!class /Script/Engine.MaterialInstanceDynamic)
  (Rendering|Material|SetScalarParameterValue _bodydynamic "FirstColor_Rough" (Utilities|Select :Index _basecolortype :NewEnumerator0 0.3 :NewEnumerator1 0.3 :NewEnumerator2 0.5) :!class /Script/Engine.MaterialInstanceDynamic)
  (Rendering|Material|SetScalarParameterValue _bodydynamic "FirstColor_Metal" (Utilities|Select :Index _basecolortype :NewEnumerator0 1.0 :NewEnumerator1 0.2 :NewEnumerator2 0.4) :!class /Script/Engine.MaterialInstanceDynamic)
  (Rendering|Material|SetScalarParameterValue _bodydynamic "FirstColor_Spec" (Utilities|Select :Index _basecolortype :NewEnumerator0 0.1 :NewEnumerator1 0.3 :NewEnumerator2 0.3) :!class /Script/Engine.MaterialInstanceDynamic)
  (Rendering|Material|SetVectorParameterValue _bodydynamic "SecondColor" (Variables|Customization|GetSecondColor) :!class /Script/Engine.MaterialInstanceDynamic)
  (Rendering|Material|SetScalarParameterValue _bodydynamic "SecondColor_Rough" (Utilities|Select :Index _secondcolortype :NewEnumerator0 0.3 :NewEnumerator1 0.3 :NewEnumerator2 0.5) :!class /Script/Engine.MaterialInstanceDynamic)
  (Rendering|Material|SetScalarParameterValue _bodydynamic "SecondColor_Metal" (Utilities|Select :Index _secondcolortype :NewEnumerator0 1.0 :NewEnumerator1 0.2 :NewEnumerator2 0.4) :!class /Script/Engine.MaterialInstanceDynamic)
  (Rendering|Material|SetScalarParameterValue _bodydynamic "SecondColor_Spec" (Utilities|Select :Index _secondcolortype :NewEnumerator0 0.1 :NewEnumerator1 0.3 :NewEnumerator2 0.3) :!class /Script/Engine.MaterialInstanceDynamic)
  (Rendering|Material|SetTextureParameterValue _bodydynamic "ColorMask" (Utilities|Select :Index (Variables|Customization|GetPaintingType) :NewEnumerator0 "/Game/ClassicBus/Textures/TX_ClassicBus_bodyMask0.TX_ClassicBus_bodyMask0" :NewEnumerator1 "/Game/ClassicBus/Textures/TX_ClassicBus_bodyMask1.TX_ClassicBus_bodyMask1" :NewEnumerator2 "/Game/ClassicBus/Textures/TX_ClassicBus_bodyMask2.TX_ClassicBus_bodyMask2" :NewEnumerator3 "/Game/ClassicBus/Textures/TX_ClassicBus_bodyMask3.TX_ClassicBus_bodyMask3"))
  (Rendering|Material|SetScalarParameterValue _bodydynamic_2 "RustIntence" (Variables|Customization|GetRust) :!class /Script/Engine.MaterialInstanceDynamic)
  (Rendering|Material|SetScalarParameterValue _bodydynamic_2 "RustContrast" (Variables|Customization|GetRustContrast) :!class /Script/Engine.MaterialInstanceDynamic)
  (Rendering|Material|SetScalarParameterValue _bodydynamic_2 "DirtContrast" (Variables|Customization|GetDirtContrast) :!class /Script/Engine.MaterialInstanceDynamic)
  (Rendering|Material|SetScalarParameterValue _bodydynamic_2 "DirtIntence" (Variables|Customization|GetDirt) :!class /Script/Engine.MaterialInstanceDynamic)
  (Rendering|Material|SetScalarParameterValue (Variables|DymamicMat|GetGlassDynamic) "Wipers" (Variables|Customization|GetGlassWipers%20) :!class /Script/Engine.MaterialInstanceDynamic)
  (Rendering|Material|SetVectorParameterValue _wheelsdynamic "Detal_Color" (Variables|Customization|GetWheelDiscColor) :!class /Script/Engine.MaterialInstanceDynamic)
  (Rendering|Material|SetScalarParameterValue _wheelsdynamic "Detal_Rough" (Utilities|Select :Index _wheeldisc :NewEnumerator0 0.3 :NewEnumerator1 0.3 :NewEnumerator2 0.5) :!class /Script/Engine.MaterialInstanceDynamic)
  (Rendering|Material|SetScalarParameterValue _wheelsdynamic "Detal_Metal" (Utilities|Select :Index _wheeldisc :NewEnumerator0 1.0 :NewEnumerator1 0.2 :NewEnumerator2 0.4) :!class /Script/Engine.MaterialInstanceDynamic)
  (Rendering|Material|SetScalarParameterValue _wheelsdynamic "Detal_Spece" (Utilities|Select :Index _wheeldisc :NewEnumerator0 0.1 :NewEnumerator1 0.3 :NewEnumerator2 0.3) :!class /Script/Engine.MaterialInstanceDynamic)
  (return))

(fn CarLights
  (params (FrontOn :type Boolean) (BackOn :type Boolean) (RightOn :type Boolean) (LeftOn :type Boolean))
  (bind _bodydynamic (Variables|DymamicMat|GetBodyDynamic))
  (Rendering|Material|SetScalarParameterValue _bodydynamic "FrontLightOn" (select FrontOn 1.0 0.0) :!class /Script/Engine.MaterialInstanceDynamic)
  (Rendering|Material|SetScalarParameterValue _bodydynamic "BackLightOn" (select BackOn 1.0 0.0) :!class /Script/Engine.MaterialInstanceDynamic)
  (Rendering|Material|SetScalarParameterValue _bodydynamic "RightLightOn" (select RightOn 1.0 0.0) :!class /Script/Engine.MaterialInstanceDynamic)
  (Rendering|Material|SetScalarParameterValue _bodydynamic "LeftLightOn" (select LeftOn 1.0 0.0) :!class /Script/Engine.MaterialInstanceDynamic)
  (return))