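; EMF zone actor for the ghost hunt that registers itself with GM_MainGame and lasts for a limited DisapationTime.
; Tick looks for an overlapping BP_TempatureZone until one is cached, then starts a one-second looping timer, apparently driving DrainHeat to lower that zone's CurrentTemp.
; Disapate, presumably the lifetime timer's callback, retries removal from the game mode's EMFZones list until it succeeds, then destroys the actor.
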(event EventBeginPlay
  (bind _asgm_main_game (Utilities|Casting|CastToGM_MainGame (Game|GetGameMode)))
  (Variables|Default|SetGameMode _asgm_main_game)
  (Utilities|Array|Add (Variables|/Game/Blueprints/GM_MainGame.GM_MainGame_C|GetEMFZones (Variables|Default|GetGameMode)) self)
  (Utilities|Time|SetTimerbyEvent (EventDispatchers|CreateEvent :!event Disapate) (Variables|Default|GetDisapationTime)))

(event EventTick
  (params (DeltaSeconds :type Float%20%28single-precision%29))
  (Variables|Default|GetIntersectingTempZone
    (:then)
    (:else
      (bind _asbp_tempature_zone (Utilities|Casting|CastToBP_TempatureZone (Utilities|Array|Get(acopy) (Collision|GetOverlappingActors "/Game/Blueprints/GhostHuntZones/BP_TempatureZone.BP_TempatureZone_C" :!class /Script/Engine.Actor))))
      (Variables|Default|SetIntersectingTempZone _asbp_tempature_zone)
      (Utilities|Time|SetTimerbyEvent (EventDispatchers|CreateEvent :!event DrainHeat) 1.0 true))))

(event Collision|EventActorBeginOverlap
  (params (OtherActor :type Actor%20Object%20Reference)))

(fn ConstructionScript)

(fn Disapate
  (bind _returnvalue (Utilities|Array|RemoveItem (Variables|/Game/Blueprints/GM_MainGame.GM_MainGame_C|GetEMFZones (Variables|Default|GetGameMode)) self :!label _label))
  (if _returnvalue
    (Actor|DestroyActor)
    (else
      (goto _label))))

(fn DrainHeat
  (bind _intersectingtempzone (Variables|Default|GetIntersectingTempZone))
  (Variables|/Game/Blueprints/GhostHuntZones/BP_TempatureZone.BP_TempatureZone_C|SetcurrentTemp _intersectingtempzone (- (Variables|/Game/Blueprints/GhostHuntZones/BP_TempatureZone.BP_TempatureZone_C|GetcurrentTemp _intersectingtempzone) (Variables|Default|GetHeatDrainAmount)))
  (return))