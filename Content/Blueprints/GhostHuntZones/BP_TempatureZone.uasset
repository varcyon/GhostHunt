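; Temperature zone actor for the ghost hunt that tracks a base temperature and a randomly fluctuating reading, with a lower floor when freezing is allowed.
; Tick recomputes the reading unless delayed; while GM_MainGame reports main power on, it also adds heat, capped at the starting temperature, and starts a timed delay.
; ResetDelay toggles the delay and zeroes the reading.
; Character overlap sets an inside-trigger flag, which is never cleared here.
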(event EventBeginPlay
  (Variables|Default|SetcurrentTemp (Variables|Default|GetstartingTemp))
  (bind _asgm_main_game (Utilities|Casting|CastToGM_MainGame (Game|GetGameMode)))
  (Variables|Default|SetGameMode _asgm_main_game))

(event Collision|EventActorBeginOverlap
  (params (OtherActor :type Actor%20Object%20Reference))
  (Utilities|Casting|CastToCharacterAvatarParent OtherActor)
  (Variables|Default|SetisInsideTrigger true))

(event EventTick
  (params (DeltaSeconds :type Float%20%28single-precision%29))
  (if (not (Variables|Default|GetonDelay))
    (CallFunction|FlucuateTemp)))

(fn ConstructionScript)

(fn FlucuateTemp
  (if (Variables|Default|GetAllowFreezing?)
    (Variables|Default|SetflucuatedTemp (+ (Math|Float|Clamp(Float) (Variables|Default|GetcurrentTemp) -2e+01 1e+02) (Math|Random|RandomFloatinRange (Variables|Default|GetflucuationMin) (Variables|Default|GetflucuationMax))))
    (else
      (Variables|Default|SetflucuatedTemp (+ (Math|Float|Clamp(Float) (Variables|Default|GetcurrentTemp) 5e+01 1e+02) (Math|Random|RandomFloatinRange (Variables|Default|GetflucuationMin) (Variables|Default|GetflucuationMax))))))
  (if (Variables|/Game/Blueprints/GM_MainGame.GM_MainGame_C|GetisMainPowerOn? (Variables|Default|GetGameMode))
    (Variables|Default|SetcurrentTemp (Math|Float|Clamp(Float) (+ (Variables|Default|GetcurrentTemp) (Variables|Default|GetRaiseHeat)) 0.0 (Variables|Default|GetstartingTemp)))
    (Variables|Default|SetonDelay true)
    (Utilities|Time|SetTimerbyEvent (EventDispatchers|CreateEvent :!event ResetDelay) (Variables|Default|GetflucuateInterval))))

(fn ResetDelay
  (Variables|Default|SetonDelay (not (Variables|Default|GetonDelay)))
  (Variables|Default|SetflucuatedTemp 0.0))