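; Base actor for an entity claw mark decal or mesh in ghost hunt zones that can dissolve in and out.
; On BeginPlay it creates a dynamic material instance of the claw mark material on its Handprint component.
; DissolveIn and DissolveOut events each play a timeline that drives the material's dissolve scalar parameter.
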(event Custom|DissolveIn
  (bind _newtrack_0 (Timeline|DissolveInTimeLine PlayFromStart)
    (:Update
      (Rendering|Material|SetScalarParameterValue (Variables|Default|GetDynamicMaterialInstance) "DissovleAmount" _newtrack_0 :!class /Script/Engine.MaterialInstanceDynamic))))

(event Custom|DissolveOut
  (bind _newtrack_0 (Timeline|DissolveOutTimeline PlayFromStart)
    (:Update
      (Rendering|Material|SetScalarParameterValue (Variables|Default|GetDynamicMaterialInstance) "DissovleAmount" _newtrack_0 :!class /Script/Engine.MaterialInstanceDynamic))))

(event EventBeginPlay
  (bind _returnvalue (Rendering|Material|CreateDynamicMaterialInstance (Variables|Default|GetHandprint) 0 "/Game/Blueprints/GhostHuntZones/ClawMark/ClawMark1_Mat1_Inst.ClawMark1_Mat1_Inst" "None" :!class /Script/Engine.PrimitiveComponent))
  (Variables|Default|SetDynamicMaterialInstance _returnvalue))

(event Collision|EventActorBeginOverlap
  (params (OtherActor :type Actor%20Object%20Reference)))

(event EventTick
  (params (DeltaSeconds :type Float%20%28single-precision%29)))

(fn ConstructionScript)