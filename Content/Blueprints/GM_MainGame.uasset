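; Main game mode that picks a random entity for the session and configures temperature zones to match its evidence.
; On BeginPlay it draws a random row from the Entities data table and stores it as the current Entity.
; It then sets AllowFreezing on every BP_TempatureZone actor, true only if one of the entity's three evidence slots holds a specific enum value.
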(event Custom|SetAllowFreezing
  (bind _entity (Variables|Default|GetEntity))
  (bind _outactors (Actor|GetAllActorsOfClass "/Game/Blueprints/GhostHuntZones/BP_TempatureZone.BP_TempatureZone_C"))
  (for _array_element _outactors
    (if (Math|Boolean|ORBoolean (Utilities|Enum|Equal(Enum) (.evidence1 _entity) "NewEnumerator8") (Utilities|Enum|Equal(Enum) (.evidence2 _entity) "NewEnumerator8") (Utilities|Enum|Equal(Enum) (.evidence3 _entity) "NewEnumerator8"))
      (Variables|/Game/Blueprints/GhostHuntZones/BP_TempatureZone.BP_TempatureZone_C|SetAllowFreezing? _array_element true)
      (else
        (Variables|/Game/Blueprints/GhostHuntZones/BP_TempatureZone.BP_TempatureZone_C|SetAllowFreezing? _array_element false)))))

(event EventBeginPlay
  (bind _outrownames (DataTable|GetDataTableRowNames (Variables|Default|GetEntities)))
  (bind _returnvalue (Utilities|GetDataTableRow "/Game/Blueprints/ParanormalEntities/Entities.Entities" (Utilities|Array|Get(acopy) _outrownames (Math|Random|RandomInteger (Utilities|Array|Length _outrownames))))
    (:then
      (Variables|Default|SetEntity _returnvalue)
      (CallFunction|SetAllowFreezing))))

(event EventTick
  (params (DeltaSeconds :type Float%20%28single-precision%29)))

(fn ConstructionScript)