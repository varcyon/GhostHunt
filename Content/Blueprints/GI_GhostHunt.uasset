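; Game instance for a ghost hunting game that handles player save data, Steam name, multiplayer sessions and the speech recognition server.
; Init loads or creates the save, launches a local ASR server process with an English model path, and fetches the Steam nickname.
; Advanced Sessions hosts open or random-code private games into the Lobby as listen server, showing error widgets on failure.
; SearchPrivateAndJoin is an empty stub.
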(event Custom|HostOpenSession
  (params (NumOfPlayers :type Integer))
  ;[1 1 1] Create Open Session
  (bind _output_get (Variables|Default|SetNumOfPlayers NumOfPlayers))
  (|AdvancedSession (Utilities|Array|MakeArray "") (Game|GetPlayerController 0) _output_get 0 false true false true true true false false false true
    (:OnSuccess
      (Game|OpenLevel(byObjectReference) "/Game/Maps/Lobby/Lobby.Lobby" true "listen"))
    (:OnFailure
      (UserInterface|CreateWidget "/Game/Maps/WB_ErrorMessage.WB_ErrorMessage_C" 0 "Failed to create session check network connection"))))

(event Custom|JoinSession
  (params (Session :type Blueprint%20Session%20Result%20Structure))
  (|JoinSession (Game|GetPlayerController 0) Session
    (:OnFailure
      (UserInterface|CreateWidget "/Game/Maps/WB_ErrorMessage.WB_ErrorMessage_C" 0 "Failed to Join session check network connection"))))

(event Custom|Start%20Speech%20Recognintion%20Server
  (Variables|Default|SetEnglishLanguageModel (Utilities|String|Append (Utilities|String|Append (Class|VoskComponent|GetProcessExecutablePath) "\\\\en-us-0.22" "SpeechRecognitionServer" "\\" "LanguageModels" "\\") "en-us-0.22"))
  (switch Utilities|FlowControl|Switch|SwitchonLanguageEnum (Variables|Default|GetLanguage)
    (:NewEnumerator0
      (Variables|Default|SetLanguageModelToUse (Variables|Default|GetEnglishLanguageModel))
      (bind (_success _returnvalue) (Class|VoskComponent|BuildServerParameters (Utilities|Struct|MakeVoskServerParameters "127.0.0.1" 8080 1 16000 0 true (Variables|Default|GetLanguageModelToUse))))
      (if _success
        (bind _processhandle (Class|VoskComponent|CreateProcess (Utilities|String|Append (Class|VoskComponent|GetProcessExecutablePath) "\\" "SpeechRecognitionServer" "\\" "asr_server.exe") _returnvalue))
        (Variables|Default|SetSpeech%20Server%20Process%20Handle _processhandle)))))

(event Custom|Kill%20Speech%20Server
  (Class|VoskComponent|KillProcess (Variables|Default|GetSpeech%20Server%20Process%20Handle)))

(event Custom|HostPrivateSession
  (params (NumOfPlayers :type Integer))
  ;[1 1 1] Create Private Session
  (bind _output_get (Variables|Default|SetNumOfPlayers NumOfPlayers))
  (|AdvancedSession (Utilities|Array|MakeArray (Class|AdvancedSessionsLibrary|MakeLiteralSessionPropertyString "PRIVATE" (Utilities|String|ToString(Integer) (Math|Random|RandomInteger 999999)))) (Game|GetPlayerController 0) _output_get 0 false true false true true true false false false true
    (:OnSuccess
      (Game|OpenLevel(byObjectReference) "/Game/Maps/Lobby/Lobby.Lobby" true "listen"))
    (:OnFailure
      (UserInterface|CreateWidget "/Game/Maps/WB_ErrorMessage.WB_ErrorMessage_C" 0 "Failed to create session check network connection"))))

(event Custom|SearchPrivateAndJoin
  (params (Session :type Integer)))

(event Custom|CheckSaveFile
  (bind _returnvalue (SaveGame|DoesSaveGameExist (Variables|Default|GetSaveSlotName)))
  (if _returnvalue
    (CallFunction|LoadPlayerData)
    (else
      (bind _returnvalue_2 (SaveGame|CreateSaveGameObject "/Game/Blueprints/SaveGameObject.SaveGameObject_C"))
      (Variables|Default|SetSaveGameData _returnvalue_2)
      (CallFunction|SavePlayerData))))

(event Custom|GetSteamName
  (if (Class|AdvancedSessionsLibrary|HasOnlineSubsystem "STEAM")
    (Utilities|FlowControl|Delay 0.2)
    (Variables|Default|SetPlayerName (Utilities|Text|ToText(String) (Class|AdvancedIdentityLibrary|GetPlayerNickname (Class|AdvancedSessionsLibrary|GetUniqueNetID (Game|GetPlayerController 0)))))))

(event EventInit
  (CallFunction|CheckSaveFile)
  (CallFunction|StartSpeechRecognintionServer)
  (CallFunction|GetSteamName))

(fn SavePlayerData
  (SaveGame|SaveGametoSlot (Variables|Default|GetSaveGameData) (Variables|Default|GetSaveSlotName)))

(fn LoadPlayerData
  (bind _returnvalue (SaveGame|LoadGamefromSlot (Variables|Default|GetSaveSlotName)))
  (bind _assave_game_object (Utilities|Casting|CastToSaveGameObject _returnvalue))
  (Variables|Default|SetSaveGameData _assave_game_object))