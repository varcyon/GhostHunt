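; Interactable notebook trigger that opens a hidden door when used.
; InteractWith marks it as usable but not grabbable, and LookAt returns the hit component with a curious prompt message.
; The Use event calls Open on the HiddenDoor reference, with no other active gameplay logic.
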(event EventBeginPlay
  (|CallParentFunction) ; This node is disabled and will not be called.\nDrag off pins to build functionality.
)

(event Collision|EventActorBeginOverlap
  (params (OtherActor :type Actor%20Object%20Reference))
  (|CallParentFunction OtherActor) ; This node is disabled and will not be called.\nDrag off pins to build functionality.
)

(event EventTick
  (params (DeltaSeconds :type Float%20%28single-precision%29))
  (|CallParentFunction DeltaSeconds) ; This node is disabled and will not be called.\nDrag off pins to build functionality.
)

(event EventUse
  (Default|Open (Variables|Default|GetHiddenDoor)))

(fn ConstructionScript
  (|CallParentFunction))

(fn Interactwith
  (params (Interactor :type Character%20Avatar%20Parent%20Object%20Reference) (HitComponent :type Primitive%20Component%20Object%20Reference) (InteractableIn :type Interactable%20Actor%20Object%20Reference))
  (return false true InteractableIn))

(fn Lookat
  (params (Interactor :type Character%20Avatar%20Parent%20Object%20Reference) (Controller :type Player%20Controller%20Object%20Reference) (HitComponent :type Primitive%20Component%20Object%20Reference))
  (return 0 HitComponent "Whats this??"))